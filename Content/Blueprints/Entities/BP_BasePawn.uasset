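; BP_BasePawn is a base pawn entity that colors itself according to its faction.
; SetFaction calls the parent implementation, then uses the faction as a row name in DT_FactionData.
; The row's color is written to the FractionColor material parameter on the skeletal mesh and selection indicator.
; The construction script applies FactionID through SetFaction, and the other events are unused stubs.
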(event EventBeginPlay)

(event Collision|EventActorBeginOverlap
  (params (OtherActor :type Actor%20Object%20Reference)))

(event EventTick
  (params (DeltaSeconds :type Float%20%28single-precision%29)))

(event EventSetFaction
  (params (NewFaction :type Integer))
  (|CallParentFunction NewFaction)
  (bind _returnvalue (Utilities|GetDataTableRow "/Game/Blueprints/DataTables/DT_FactionData.DT_FactionData" (Utilities|String|StringToName (Utilities|String|ToString(Integer) NewFaction)))
    (:then
      (Rendering|Material|SetVectorParameterValueonMaterials (Variables|Default|GetSkeletalMesh) "FractionColor" (Math|Conversions|ToVector(LinearColor) (.Color (Utilities|Struct|BreakMRC_FactionData _returnvalue)))))))

(fn ConstructionScript
  (Class|MRCFactionInterface|SetFaction (Variables|Default|GetFactionID)))