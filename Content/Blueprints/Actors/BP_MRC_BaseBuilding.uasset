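; Base building actor Blueprint that tints itself by faction and shows placement validity.
; SetFaction, also run from the construction script, calls its parent, then reads the faction's color from DT_FactionData.
; That color feeds material parameters on the static mesh and selection indicator.
; ToggleBuildingValidity drives the mesh's "Invalid" material scalar, which becomes 1 when Valid is true, despite the parameter's name.
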(event EventSetFaction
  (params (NewFaction :type Integer))
  ;[0.15 0.15 0.15 0.5] Set Faction Colors
  (|CallParentFunction NewFaction)
  (bind _returnvalue (Utilities|GetDataTableRow "/Game/Blueprints/DataTables/DT_FactionData.DT_FactionData" (Utilities|String|StringToName (Utilities|String|ToString(Integer) NewFaction)))
    (:then
      (Rendering|Material|SetVectorParameterValueonMaterials (Variables|Default|GetSelectedIndicator) "FractionColor" (Math|Conversions|ToVector(LinearColor) (.Color (Utilities|Struct|BreakMRC_FactionData _returnvalue))))
      (Rendering|Material|SetVectorParameterValueonMaterials (Variables|Default|GetStaticMesh) "Player Color" (Math|Conversions|ToVector(LinearColor) (.Color (Utilities|Struct|BreakMRC_FactionData _returnvalue)))))))

(event EventToggleBuildingValidity
  (params (bValid :type Boolean))
  ;[0.15 0.15 0.15 0.5] Show Placement Validation
  (Rendering|Material|SetScalarParameterValueonMaterials (Variables|Default|GetStaticMesh) "Invalid" (Math|Float|SelectFloat 1.0 0.0 bValid)))

(fn ConstructionScript
  (Class|MRCFactionInterface|SetFaction (Variables|Default|GetFactionID)))