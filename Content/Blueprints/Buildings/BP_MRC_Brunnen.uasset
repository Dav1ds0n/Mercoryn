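; BP_MRC_Brunnen is a clickable building actor for a well ("Brunnen").
; Clicking its StaticMesh prints "Brunnen" as debug text and calls PlayMontage, with no montage or target visible in the graph.
; An actor-level OnClicked binding with an empty handler is left unconnected and never runs.
; BeginPlay, overlap and Tick are disabled stubs, and the construction script only calls its parent.
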(event OnClicked(StaticMesh)
  (params (TouchedComponent :type Primitive%20Component%20Object%20Reference) (ButtonPressed :type Key%20Structure))
  (Development|PrintString "Brunnen")
  (Animation|Montage|PlayMontage 0 0))

(event Custom|OnClicked_Event
  (params (TouchedActor :type Actor%20Object%20Reference) (ButtonPressed :type Key%20Structure :default "None")))

(event EventBeginPlay
  (|CallParentFunction) ; Dieser Knoten ist deaktiviert und wird nicht aufgerufen.\nZiehe die Pins ab, um die Funktionalität aufzubauen.
)

(event Collision|EventActorBeginOverlap
  (params (OtherActor :type Actor%20Object%20Reference))
  (|CallParentFunction OtherActor) ; Dieser Knoten ist deaktiviert und wird nicht aufgerufen.\nZiehe die Pins ab, um die Funktionalität aufzubauen.
)

(event EventTick
  (params (DeltaSeconds :type Float%20%28single-precision%29))
  (|CallParentFunction DeltaSeconds) ; Dieser Knoten ist deaktiviert und wird nicht aufgerufen.\nZiehe die Pins ab, um die Funktionalität aufzubauen.
)

(fn ConstructionScript
  (|CallParentFunction))